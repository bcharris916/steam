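; Lobby game mode that manages players, character selection and map settings before server-traveling to one of two arena maps.
; On login it initializes each lobby controller and possesses a base pawn at a random PlayerStart; SwapCharacter replaces that pawn.
; EveryoneUpdate, run on respawn and logout, rebuilds and pushes player info and available characters, and sets CanWeStart from character choices.
; It also pushes map changes to all controllers and handles kicks.
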(event Custom|SwapCharacter
  (params (playerController :type Player%20Controller%20Object%20Reference) (characterClass :type Character%20Class%20Reference) (changedStatus :type Boolean))
  (bind _returnvalue (Pawn|GetControlledPawn playerController))
  (bind _spawnpoints (Variables|Default|GetspawnPoints))
  ;[1 1 1] Swaps current character with selected charcater from character select screen
  (if (not changedStatus)
    (Utilities|IsValid _returnvalue
      (:Is%20Valid
        (Actor|DestroyActor _returnvalue))
      (:Is%20Not%20Valid
        _))
    (bind _returnvalue_2 (Game|SpawnActorfromClass characterClass (Transformation|GetActorTransform (Utilities|Array|Get(acopy) _spawnpoints (Math|Random|RandomIntegerinRange 0 (- (Utilities|Array|Length _spawnpoints) 1)))) "AlwaysSpawn" 0 0))
    (Pawn|Possess playerController _returnvalue_2)))

(event Custom|launchGame
  (bind _returnvalue (Game|GetPlayerController 0))
  ;[1 1 1] Launch game based off map settings
  (switch int (Variables|Default|GetgmMapID)
    (:0
      (Development|ExecuteConsoleCommand "servertravel /Game/Maps/Arena01" _returnvalue))
    (:1
      (Development|ExecuteConsoleCommand "servertravel /Game/Maps/Arena02" _returnvalue))))

(event Custom|everyoneUpdate
  (bind _allplayercontrollers (Variables|Default|GetallPlayerControllers))
  ;[1 1 1] updates al connected players lobby info when called
  (bind _output_get (Variables|Default|SetcurrentPlayers (Utilities|Array|Length (Variables|Default|GetallPlayerControllers))))
  (if (> _output_get 0)
    (Utilities|Array|Clear (Variables|Default|GetconnectedPlayers))
    (for _array_element _allplayercontrollers
      (bind _aslobby_player_controller (Utilities|Casting|CastTolobbyPlayerController _array_element))
      (Utilities|Array|Add (Variables|Default|GetconnectedPlayers) (Variables|/Game/Blueprints/lobby/lobbyPlayerController.lobbyPlayerController_C|GetplayerSettings _aslobby_player_controller))
      (Default|UpdateNumPlayers _aslobby_player_controller (Variables|Default|GetcurrentPlayers) (Variables|Default|GetmaxPlayers)))
    (for _array_element_2 _allplayercontrollers
      (bind _aslobby_player_controller_2 (Utilities|Casting|CastTolobbyPlayerController _array_element_2))
      (Default|AddPlayerInfo _aslobby_player_controller_2 (Variables|Default|GetconnectedPlayers))
      (Default|UpdateAvalableCharacters _aslobby_player_controller_2 (Variables|Default|GetavailableCharacters))
      (CallFunction|AddtoKickList))
    (bind _array_element_3 (Utilities|Array|ForEachLoopwithBreak (Variables|Default|GetconnectedPlayers))
      (:LoopBody
        (if (== (.myPlayerCharacter (Utilities|Struct|BreakPlayerInfo _array_element_3)) "/Game/Blueprints/characters/0_base.0_base_C")
          (Variables|Default|SetcanWeStart? false)
          (CallFunction|CannotStartGame)
          (else
            (Variables|Default|SetcanWeStart? true)))))))

(event Custom|addToKickList
  ;[1 1 1] add to kick list if game settings is open
  (bind _aslobby_player_controller (Utilities|Casting|CastTolobbyPlayerController (Game|GetPlayerController 0)))
  (Utilities|IsValid (Variables|/Game/Blueprints/lobby/lobbyPlayerController.lobbyPlayerController_C|GetlobbyMenuWB _aslobby_player_controller)
    (:Is%20Valid
      (if (Widget|IsVisible (Variables|/Game/UI/Lobby/lobbyMenu.lobbyMenu_C|GetgameSettings (Variables|/Game/Blueprints/lobby/lobbyPlayerController.lobbyPlayerController_C|GetlobbyMenuWB _aslobby_player_controller)))
        (Default|FillPlayersWindow (Variables|/Game/UI/Lobby/lobbyMenu.lobbyMenu_C|GetgameSettings (Variables|/Game/Blueprints/lobby/lobbyPlayerController.lobbyPlayerController_C|GetlobbyMenuWB _aslobby_player_controller)))))))

(event Custom|cannotStartGame)

(event Custom|serverUpdateGameSettings
  (params (mapImage :type Texture%202D%20Object%20Reference) (mapName :type Text) (mapTime :type Text) (mapID :type Integer))
  ;[1 1 1] Server has made changes.  tell the client to update their lobby info
  (Variables|Default|SetgmMapImage mapImage)
  (Variables|Default|SetgmMapName mapName)
  (Variables|Default|SetgmMapTime mapTime)
  (Variables|Default|SetgmMapID mapID)
  (for _array_element (Variables|Default|GetallPlayerControllers)
    (bind _aslobby_player_controller (Utilities|Casting|CastTolobbyPlayerController _array_element))
    (Default|UpdateLobbySettings _aslobby_player_controller (Variables|Default|GetgmMapImage) (Variables|Default|GetgmMapName) (Variables|Default|GetgmMapTime))))

(event Custom|youHaveBeenKicked
  (params (playerID :type Integer))
  ;[1 1 1] Kick the Selected Players From Lobby
  (Default|Kicked (.AsLobby%20Player%20Controller (Utilities|Casting|CastTolobbyPlayerController (Utilities|Array|Get(acopy) (Variables|Default|GetallPlayerControllers) playerID)))))

(event Custom|respawnPlayer
  (params (playerController :type Player%20Controller%20Object%20Reference))
  (bind _returnvalue (Pawn|GetControlledPawn playerController))
  (bind _spawnpoints (Variables|Default|GetspawnPoints))
  ;[1 1 1] Spawn player as base character when arriving at the lobby. tells everyone to update their lobbies
  (Utilities|IsValid _returnvalue
    (:Is%20Valid
      (Actor|DestroyActor _returnvalue))
    (:Is%20Not%20Valid
      _))
  (bind _returnvalue_2 (Game|SpawnActorfromClass "/Game/Blueprints/characters/0_base.0_base_C" (Transformation|GetActorTransform (Utilities|Array|Get(acopy) _spawnpoints (Math|Random|RandomIntegerinRange 0 (- (Utilities|Array|Length _spawnpoints) 1)))) "AdjustIfPossibleButAlwaysSpawn" 0 0))
  (Pawn|Possess playerController _returnvalue_2)
  (CallFunction|EveryoneUpdate))

(event EventPostLogin
  (params (NewPlayer :type Player%20Controller%20Object%20Reference))
  ;[1 1 1] Initial Setup happens on Event Post Login handles lobby setup on plaeyr controller and spawn player
  (Networking|SwitchHasAuthority
    (:Authority
      (Utilities|Array|Add (Variables|Default|GetallPlayerControllers) NewPlayer)
      (bind _outactors (Actor|GetAllActorsOfClass "/Script/Engine.PlayerStart"))
      (Variables|Default|SetspawnPoints _outactors)
      (bind _asgame_info_instance (Utilities|Casting|CastTogameInfoInstance (Game|GetGameInstance)))
      (Variables|Default|SetserverName (Variables|/Game/Blueprints/allLevels/gameInfoInstance.gameInfoInstance_C|GetserverName _asgame_info_instance))
      (Variables|Default|SetmaxPlayers (Variables|/Game/Blueprints/allLevels/gameInfoInstance.gameInfoInstance_C|GetmaxPlayers _asgame_info_instance))
      (bind _aslobby_player_controller (Utilities|Casting|CastTolobbyPlayerController NewPlayer)
        (:then
          (Default|InitalSetup _aslobby_player_controller)
          (Default|SetupLobbyMenu _aslobby_player_controller (Variables|Default|GetserverName))
          (Default|UpdateLobbySettings _aslobby_player_controller (Variables|Default|GetgmMapImage) (Variables|Default|GetgmMapName) (Variables|Default|GetgmMapTime))
          (CallFunction|RespawnPlayer NewPlayer))
        (:CastFailed
          (Development|PrintString "Loading charcter failed to cast to lobby player controller"))))))

(event EventOnLogout
  (params (ExitingController :type Controller%20Object%20Reference))
  (bind _allplayercontrollers (Variables|Default|GetallPlayerControllers))
  ;[1 1 1] Event on logout removes player controller and connected player info and resets available character
  (bind (_array_element _array_index) (Utilities|Array|ForEachLoopwithBreak _allplayercontrollers :!label _label)
    (:LoopBody
      (if (== _array_element ExitingController)
        (goto _label Break)))
    (:Completed
      (bind _aslobby_player_controller (Utilities|Casting|CastTolobbyPlayerController (Utilities|Array|Get(acopy) _allplayercontrollers _array_index)))
      (Utilities|Array|SetArrayElem (Variables|Default|GetavailableCharacters) (Variables|/Game/Blueprints/lobby/lobbyPlayerController.lobbyPlayerController_C|GetselectedCharacter _aslobby_player_controller) false)
      (Utilities|Array|RemoveIndex (Variables|Default|GetallPlayerControllers) _array_index)
      (Utilities|Array|RemoveIndex (Variables|Default|GetconnectedPlayers) _array_index)
      (CallFunction|EveryoneUpdate))))

(fn ConstructionScript)