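; Attack component that resolves an attack key into one of the attacks held in two switchable sets.
; GetSelectedAttack uses the AisSelected flag to choose AttacksA or AttacksB, then maps keys A through D to that array's first four entries.
; ProcessAttackRequest only performs this lookup and does nothing with the result.
; GetAttackAvailability is an empty stub, with an unconnected read of the attack's last-use time.
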(event EventBeginPlay)

(event EventTick
  (params (DeltaSeconds :type Float%20%28single-precision%29)))

(fn ProcessAttackRequest
  (params (AttackKey :type AttackKeys%20Enum :default "NewEnumerator0"))
  (CallFunction|GetSelectedAttack AttackKey))

(fn GetSelectedAttack
  (params (attackKey :type AttackKeys%20Enum :default "NewEnumerator0"))
  (bind _attacksb (Variables|Default|GetAttacksB))
  (if (Variables|Default|GetAisSelected)
    (switch Utilities|FlowControl|Switch|SwitchonAttackKeys attackKey
      (:NewEnumerator0
        (return (Utilities|Array|Get(acopy) (Variables|Default|GetAttacksA))))
      (:NewEnumerator1
        (return (Utilities|Array|Get(acopy) (Variables|Default|GetAttacksA) 1)))
      (:NewEnumerator2
        (return (Utilities|Array|Get(acopy) (Variables|Default|GetAttacksA) 2)))
      (:NewEnumerator3
        (return (Utilities|Array|Get(acopy) (Variables|Default|GetAttacksA) 3))))
    (else
      (switch Utilities|FlowControl|Switch|SwitchonAttackKeys attackKey
        (:NewEnumerator0
          (return (Utilities|Array|Get(acopy) _attacksb)))
        (:NewEnumerator1
          (return (Utilities|Array|Get(acopy) _attacksb 1)))
        (:NewEnumerator2
          (return (Utilities|Array|Get(acopy) _attacksb 2)))
        (:NewEnumerator3
          (return (Utilities|Array|Get(acopy) _attacksb 3)))))))

(fn GetAttackAvailability
  (params (attack :type Attack%20Object%20Reference)))