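; Example-map bot for the fog of war system that wanders between preset points.
; On BeginPlay it converts LocalLocations to world space through its own transform, then every two seconds issues a SimpleMoveToLocation to a randomly chosen one.
; The construction script uses Type to pair a mesh color with FOWComponent settings: green is not hidden in fog, red is hidden, and blue is hidden with its location remembered.
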(event EventBeginPlay
  (bind _globallocations (Variables|Default|GetGlobalLocations))
  (for _array_element (Variables|Default|GetLocalLocations)
    (Utilities|Array|Add (Variables|Default|GetGlobalLocations) (Math|Transform|TransformLocation (Transformation|GetActorTransform) _array_element)))
  (AI|Navigation|SimpleMovetoLocation (Pawn|GetController) (Utilities|Array|Get(acopy) _globallocations (Math|Random|RandomIntegerinRange 0 (- (Utilities|Array|Length _globallocations) 1))) :!label _label)
  (Utilities|FlowControl|Delay 2.0)
  (goto _label))

(fn ConstructionScript
  (bind _mesh (Variables|Character|GetMesh))
  (bind _fowcomponent (Variables|Default|GetFOWComponent))
  (switch Utilities|FlowControl|Switch|SwitchonVisibilityMode (Variables|Default|GetType)
    (:NewEnumerator0
      (Rendering|Material|SetMaterial _mesh 0 "/Game/FogOfWar/ExampleMap/Materials/SimpleGreen.SimpleGreen")
      (Variables|/Game/FogOfWar/Blueprints/FOWComponent.FOWComponent_C|SetHideInFOW _fowcomponent false)
      (Variables|/Game/FogOfWar/Blueprints/FOWComponent.FOWComponent_C|SetRememberLocation _fowcomponent false))
    (:NewEnumerator1
      (Rendering|Material|SetMaterial _mesh 0 "/Game/FogOfWar/ExampleMap/Materials/SimpleRed.SimpleRed")
      (Variables|/Game/FogOfWar/Blueprints/FOWComponent.FOWComponent_C|SetHideInFOW _fowcomponent true)
      (Variables|/Game/FogOfWar/Blueprints/FOWComponent.FOWComponent_C|SetRememberLocation _fowcomponent false))
    (:NewEnumerator2
      (Rendering|Material|SetMaterial _mesh 0 "/Game/FogOfWar/ExampleMap/Materials/SimpleBlue.SimpleBlue")
      (Variables|/Game/FogOfWar/Blueprints/FOWComponent.FOWComponent_C|SetHideInFOW _fowcomponent true)
      (Variables|/Game/FogOfWar/Blueprints/FOWComponent.FOWComponent_C|SetRememberLocation _fowcomponent true))))