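; Example-map bot actor that demonstrates fog of war visibility behaviors through its FOWComponent.
; The construction script switches on the Type enum to set both the mesh color and the component's flags.
; Green stays visible in fog, red hides in fog, and blue hides in fog with location memory enabled.
; The event graph has no active logic.
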(event EventBeginPlay)

(event EventActorBeginOverlap
  (params (OtherActor :type Actor%20Object%20Reference)))

(event EventTick
  (params (DeltaSeconds :type Float%20%28single-precision%29)))

(fn ConstructionScript
  (bind _mesh (Variables|Character|GetMesh))
  (bind _fowcomponent (Variables|Default|GetFOWComponent))
  (switch Utilities|FlowControl|Switch|SwitchonVisibilityMode (Variables|Default|GetType)
    (:NewEnumerator0
      (Rendering|Material|SetMaterial _mesh 0 "/Game/FogOfWar/ExampleMap/Materials/SimpleGreen.SimpleGreen")
      (Variables|/Game/FogOfWar/Blueprints/FOWComponent.FOWComponent_C|SetHideInFOW _fowcomponent false)
      (Variables|/Game/FogOfWar/Blueprints/FOWComponent.FOWComponent_C|SetRememberLocation _fowcomponent false))
    (:NewEnumerator1
      (Rendering|Material|SetMaterial _mesh 0 "/Game/FogOfWar/ExampleMap/Materials/SimpleRed.SimpleRed")
      (Variables|/Game/FogOfWar/Blueprints/FOWComponent.FOWComponent_C|SetHideInFOW _fowcomponent true)
      (Variables|/Game/FogOfWar/Blueprints/FOWComponent.FOWComponent_C|SetRememberLocation _fowcomponent false))
    (:NewEnumerator2
      (Rendering|Material|SetMaterial _mesh 0 "/Game/FogOfWar/ExampleMap/Materials/SimpleBlue.SimpleBlue")
      (Variables|/Game/FogOfWar/Blueprints/FOWComponent.FOWComponent_C|SetHideInFOW _fowcomponent true)
      (Variables|/Game/FogOfWar/Blueprints/FOWComponent.FOWComponent_C|SetRememberLocation _fowcomponent true))))