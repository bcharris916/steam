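; Example-map wall actor that repeatedly switches its fog of war casting on and off.
; From BeginPlay it loops endlessly with two-second delays, toggling CastFOW on its FOWComponent.
; Each toggle also sets the cube's response on the GameTraceChannel1 collision channel to Ignore or Block, matching the casting state.
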(event EventBeginPlay
  (bind _fowcomponent (Variables|Default|GetFOWComponent))
  (Utilities|FlowControl|Delay 2.0 :!label _label)
  (Variables|/Game/FogOfWar/Blueprints/FOWComponent.FOWComponent_C|SetCastFOW _fowcomponent false)
  (Collision|SetCollisionResponsetoChannel (Variables|Default|GetCube) "ECC_GameTraceChannel1" "ECR_Ignore")
  (Utilities|FlowControl|Delay 2.0)
  (Variables|/Game/FogOfWar/Blueprints/FOWComponent.FOWComponent_C|SetCastFOW _fowcomponent true)
  (Collision|SetCollisionResponsetoChannel (Variables|Default|GetCube) "ECC_GameTraceChannel1" "ECR_Block")
  (goto _label))

(fn ConstructionScript
  (|CallParentFunction))